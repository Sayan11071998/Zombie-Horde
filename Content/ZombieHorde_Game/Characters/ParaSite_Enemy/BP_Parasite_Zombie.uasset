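; Parasite zombie enemy that endlessly chases player 0 and attacks it on reaching range.
; A self-restarting AI MoveTo loop deals damage through BP_Player's TakeDamage, gated by a CanAttack flag that RechargeAttack resets after AttackRate.
; DealDamage lowers Health and, at zero, ragdolls the mesh, stops the chase, increments the player's kill count and destroys the actor after a short delay.
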(event `Recharge Attack`
  ;[1 1 1] Recharge Attack
  (`KismetSystemLibrary.Delay` (`self.Attack Rate`))
  (set `self.CanAttack` true))

(event `Chase Player`
  ;[1 1 1] Enemy AI
  (if (not (`self.EnemyDied`))
    (`|AIMoveTo` self (0.0 0.0 0.0) (`GameplayStatics.GetPlayerCharacter` 0) 100.0
      (:`OnSuccess`
        (if (`self.CanAttack`)
          (set `self.CanAttack` false)
          (`self.Recharge Attack`)
          (`self.Chase Player`)
          (bind _asbp_player (cast `/Game/ZombieHorde_Game/Characters/Player_Character/BP_Player` (`GameplayStatics.GetPlayerCharacter` 0)))
          (`/Game/ZombieHorde_Game/Characters/Player_Character/BP_Player.Take Damage` _asbp_player (`self.Damage To Do`))
          (else
            (`self.Chase Player`))))
      (:`OnFail`
        (`self.Chase Player`)))))

(event `self.ReceiveBeginPlay`
  (set `self.Health` (`self.Max Health`))
  (`KismetSystemLibrary.Delay` 0.2)
  (`self.Chase Player`))

(event `Deal Damage`
  (params (Damage :type "Float (double-precision)"))
  ;[1 1 1] Deal Damage
  (bind _output_get (set `self.Health` (- (`self.Health`) Damage)))
  (if (<= _output_get 0.0)
    (`PrimitiveComponent.SetSimulatePhysics` (`self.Mesh`) true)
    (set `self.EnemyDied` true)
    (bind _asbp_player (cast `/Game/ZombieHorde_Game/Characters/Player_Character/BP_Player` (`GameplayStatics.GetPlayerCharacter` 0)))
    (`/Game/ZombieHorde_Game/Characters/Player_Character/BP_Player.Increment Kill Count` _asbp_player)
    (`KismetSystemLibrary.Delay` 1.0)
    (`self.K2_DestroyActor`)
    (set `self.Damage To Do` 0.0)))

(fn `UserConstructionScript`)