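; Zombie enemy that endlessly chases the player and deals damage on reaching them, with a cooldown between attacks.
; A self-restarting AIMoveTo loop drives the chase, starting just after spawn so the navmesh is found.
; DealDamage awards score for non-lethal body hits, while head hits kill instantly and hide the head bone.
; Death ragdolls the mesh, removes the capsule, credits score and one kill, then destroys the actor after a delay.
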(event `Chase Player`
  ;[1 1 1] Chase Player
  (`|AIMoveTo` self (0.0 0.0 0.0) (`GameplayStatics.GetPlayerCharacter` 0)
    (:`OnSuccess`
      (if (`self.CanAttack`)
        (set `self.CanAttack` false)
        (`self.RechargeAttack`)
        (`self.Chase Player`)
        (bind _asbp_player (cast `/Game/Blueprints/Characters/Player/BP_Player` (`GameplayStatics.GetPlayerCharacter` 0)))
        (`/Game/Blueprints/Characters/Player/BP_Player.Take Damage` _asbp_player (`self.Damage To Do`))
        (else
          (`self.Chase Player`))))
    (:`OnFail`
      (`self.Chase Player`))))

(event `RechargeAttack`
  ;[1 1 1] Chase Player
  (`KismetSystemLibrary.Delay` (`self.AttackRate`))
  (set `self.CanAttack` true))

(event `self.ReceiveBeginPlay`
  (set `self.Health` (`self.MaxHealth`))
  ;[1 1 1] Chase ( delay to let new zombies find nav)
  (`KismetSystemLibrary.Delay` 0.01)
  (`self.Chase Player`))

(event `/Game/Blueprints/Interfaces/BPI_Weapon.DealDamage`
  (params (Damage :type "Float (double-precision)") (SocketHit :type Name))
  (bind _capsulecomponent (`self.CapsuleComponent`))
  (bind _capsulecomponent_2 (`self.CapsuleComponent`))
  (set `self.Health - Damage` (- (`self.Health`) Damage))
  (if (== SocketHit "head")
    (set `self.Health - Damage` 0.0)
    (`SkinnedMeshComponent.HideBoneByName` (`self.Mesh`) "head" "PBO_None")
    (`|ExecutionSequence`
      (:`then_0`
        (set `self.Health` 0.0)
        (`PrimitiveComponent.SetSimulatePhysics` (`self.Mesh`) true)
        (`|ExecutionSequence`
          (:`then_0`
            (`/Engine/EditorBlueprintResources/StandardMacros.IsValid` _capsulecomponent
              (:`Is Valid`
                (`ActorComponent.K2_DestroyComponent` _capsulecomponent))))
          (:`then_1`
            (`/Engine/EditorBlueprintResources/StandardMacros.DoOnce` false
              (:`Completed`
                (bind _asbp_player (cast `/Game/Blueprints/Characters/Player/BP_Player` (`GameplayStatics.GetPlayerCharacter` 0)))
                (set `/Game/Blueprints/Characters/Player/BP_Player.KillCounter` (+ (`/Game/Blueprints/Characters/Player/BP_Player.KillCounter` _asbp_player) 1) _asbp_player)
                (set `/Game/Blueprints/Characters/Player/BP_Player.Score` (+ (`/Game/Blueprints/Characters/Player/BP_Player.Score` _asbp_player) (`self.HeadshotScore`)) _asbp_player))))))
      (:`then_1`
        (`KismetSystemLibrary.Delay` (`self.Time Until Destroy`))
        (`self.K2_DestroyActor`)))
    (else
      ;[1 1 1] Death
      (if (> (`self.Health - Damage`) 0.0)
        (set `self.Health` (`self.Health - Damage`))
        (bind _asbp_player_2 (cast `/Game/Blueprints/Characters/Player/BP_Player` (`GameplayStatics.GetPlayerCharacter` 0)))
        (set `/Game/Blueprints/Characters/Player/BP_Player.Score` (+ (`/Game/Blueprints/Characters/Player/BP_Player.Score` _asbp_player_2) (`self.HitScore`)) _asbp_player_2)
        (else
          (`|ExecutionSequence`
            (:`then_0`
              (set `self.Health` 0.0)
              (`PrimitiveComponent.SetSimulatePhysics` (`self.Mesh`) true)
              (`|ExecutionSequence`
                (:`then_0`
                  (`/Engine/EditorBlueprintResources/StandardMacros.IsValid` _capsulecomponent_2
                    (:`Is Valid`
                      (`ActorComponent.K2_DestroyComponent` _capsulecomponent_2))))
                (:`then_1`
                  (`/Engine/EditorBlueprintResources/StandardMacros.DoOnce` false
                    (:`Completed`
                      (bind _asbp_player_3 (cast `/Game/Blueprints/Characters/Player/BP_Player` (`GameplayStatics.GetPlayerCharacter` 0)))
                      (set `/Game/Blueprints/Characters/Player/BP_Player.KillCounter` (+ (`/Game/Blueprints/Characters/Player/BP_Player.KillCounter` _asbp_player_3) 1) _asbp_player_3)
                      (set `/Game/Blueprints/Characters/Player/BP_Player.Score` (+ (`/Game/Blueprints/Characters/Player/BP_Player.Score` _asbp_player_3) (`self.HitScore`)) _asbp_player_3))))))
            (:`then_1`
              (`KismetSystemLibrary.Delay` (`self.Time Until Destroy`))
              (`self.K2_DestroyActor`))))))))

(fn `UserConstructionScript`)